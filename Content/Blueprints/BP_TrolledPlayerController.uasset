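; Player controller that owns and manages the game's UI: HUD, map, inventory, pause menu, loot menu, notifications and death screen.
; Most widgets are created lazily on first use and cached, with the inventory pre-built on BeginPlay and the loot menu rebuilt on each show.
; Map shows while held; inventory switches to UI-only input with a cursor.
; ShowIngameUI rebuilds HUD and notifications for local controllers, while events trigger hit markers and messages.
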(event Custom|Create%20Notification%20UI
  ;[1 1 1] Notifications from server (Cant equip, consume, etc.)
  (Utilities|IsValid (Variables|Default|GetNotificationWidget)
    (:Is%20Valid
      _)
    (:Is%20Not%20Valid
      (bind _returnvalue (UserInterface|CreateWidget "/Game/UserInterface/Widgets/WBP_NotificationStack.WBP_NotificationStack_C"))
      (bind _output_get (Variables|Default|SetNotificationWidget _returnvalue))))
  (UserInterface|Viewport|AddtoViewport _output_get 0))

(event Custom|Open%20Pause%20Menu
  ;[1 1 1] Open Pause Menu
  (Variables|Default|GetPauseWidget
    (:then
      _)
    (:else
      (bind _returnvalue (UserInterface|CreateWidget "/Game/UserInterface/Widgets/WBP_PauseMenu.WBP_PauseMenu_C"))
      (bind _output_get (Variables|Default|SetPauseWidget _returnvalue))))
  (UserInterface|Viewport|AddtoViewport _output_get 0))

(event Custom|Add%20HUD
  ;[1 1 1] Main HUD
  (Utilities|IsValid (Variables|Default|GetMainWidget)
    (:Is%20Valid
      _)
    (:Is%20Not%20Valid
      (bind _returnvalue (UserInterface|CreateWidget "/Game/UserInterface/Widgets/WBP_Main.WBP_Main_C"))
      (bind _output_get (Variables|Default|SetMainWidget _returnvalue))))
  (UserInterface|Viewport|AddtoViewport _output_get 0))

(event Custom|Close%20Pause%20Menu
  ;[1 1 1] Close Pause Menu
  (bind _pausewidget (Variables|Default|GetPauseWidget)
    (:then
      (Widget|RemovefromParent _pausewidget))
    (:else)))

(event EventShowDeathScreen
  (params (Killer :type Main%20Character%20Object%20Reference))
  (Viewport|RemoveAllWidgets)
  (Variables|Default|GetDeathWidget
    (:then
      _)
    (:else
      (bind _returnvalue (UserInterface|CreateWidget "/Game/UserInterface/Widgets/WBp_DeathScreen.WBP_DeathScreen_C" 0 Killer))
      (bind _output_get (Variables|Default|SetDeathWidget _returnvalue))))
  (UserInterface|Viewport|AddtoViewport _output_get 0))

(event EventShowIngameUI
  ;[1 1 1] Draw All UI
  (if (Pawn|IsLocalPlayerController)
    (Viewport|RemoveAllWidgets)
    (CallFunction|AddHUD)
    (CallFunction|CreateNotificationUI)))

(event EventShowNotification
  (params (Message :type Text%20%28by%20ref%29))
  (bind _notificationwidget (Variables|Default|GetNotificationWidget))
  ;[1 1 1] Show event notification
  (Utilities|IsValid _notificationwidget
    (:Is%20Valid
      (Default|AddNotification _notificationwidget Message))))

(event EventShowLootMenu
  (params (LootSource :type Inventory%20Component%20Object%20Reference))
  ;[1 1 1] Show/Hide loot menu
  (Utilities|IsValid LootSource
    (:Is%20Valid
      (bind _returnvalue (UserInterface|CreateWidget "/Game/UserInterface/Widgets/WBP_LootMenu.WBP_LootMenu_C"))
      (bind _output_get (Variables|Default|SetLootMenuWidget _returnvalue))
      (UserInterface|Viewport|AddtoViewport _output_get 0))))

(event EventHideLootMenu
  ;[1 1 1] Show/Hide loot menu
  (Widget|RemovefromParent (Variables|Default|GetLootMenuWidget)))

(event EventOnHitPlayer
  (bind _mainwidget (Variables|Default|GetMainWidget))
  ;[1 1 1] Show hit marker
  (UserInterface|Animation|PlayAnimation _mainwidget (Variables|/Game/UserInterface/Widgets/WBP_Main.WBP_Main_C|GetHitmarkerAnim _mainwidget) 0.0 1 "Forward" 1.0 false))

(event EventBeginPlay
  ;[1 1 1] Construct inventory on begin play
  (Utilities|IsValid (Variables|Default|GetInventoryWidget)
    (:Is%20Not%20Valid
      (bind _returnvalue (UserInterface|CreateWidget "/Game/UserInterface/Widgets/WBP_Inventory.WBP_Inventory_C"))
      (Variables|Default|SetInventoryWidget _returnvalue)
      (Input|SetInputModeGameOnly self)
      (Variables|Default|SetbShowMouseCursor false))))

(event Input|ActionEvents|InputActionInventory
  (params (Key :type Key%20Structure :default "None"))
  ;[1 1 1] Inventory
  (:Pressed
    (Utilities|IsValid (Variables|Default|GetInventoryWidget)
      (:Is%20Valid
        _)
      (:Is%20Not%20Valid
        (bind _returnvalue (UserInterface|CreateWidget "/Game/UserInterface/Widgets/WBP_Inventory.WBP_Inventory_C"))
        (bind _output_get (Variables|Default|SetInventoryWidget _returnvalue))))
    (UserInterface|Viewport|AddtoViewport _output_get 0)
    (Variables|Default|SetbShowMouseCursor true)
    (Input|SetInputModeUIOnly self _output_get "DoNotLock")))

(event Input|ActionEvents|InputActionMap
  (params (Key :type Key%20Structure :default "None"))
  ;[1 1 1] Open/Close Map
  (:Pressed
    (Utilities|IsValid (Variables|Default|GetMapWidget)
      (:Is%20Valid
        _)
      (:Is%20Not%20Valid
        (bind _returnvalue (UserInterface|CreateWidget "/Game/UserInterface/Widgets/WBP_Map.WBP_Map_C" self))
        (bind _output_get (Variables|Default|SetMapWidget _returnvalue))))
    (UserInterface|Viewport|AddtoViewport _output_get 0))
  (:Released
    (Widget|RemovefromParent (Variables|Default|GetMapWidget))))

(event Input|ActionEvents|InputActionPause
  (params (Key :type Key%20Structure :default "None"))
  ;[1 1 1] Open Pause Menu
  (:Pressed
    (CallFunction|OpenPauseMenu)))

(fn ConstructionScript)