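; Game mode for Trolled that assigns each joining player a random, unused spawn point.
; BeginPlay caches every BP_Trolled_PlayerStart actor in the level into PlayerStarts.
; FindPlayerStart re-rolls a random entry until it finds one not Used, then marks and returns it, with no exit if all are taken.
; Selection ignores distance to other players, which a comment flags for improvement.
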(event EventBeginPlay
  (bind _outactors (Actor|GetAllActorsOfClass "/Game/Blueprints/BP_Trolled_PlayerStart.BP_Trolled_PlayerStart_C"))
  (Variables|Default|SetPlayerStarts _outactors))

(event EventTick
  (params (DeltaSeconds :type Float%20%28single-precision%29)))

(fn ConstructionScript)

(fn FindPlayerStart
  (params (Player :type Controller%20Object%20Reference) (IncomingName :type String))
  (bind _playerstarts (Variables|Default|GetPlayerStarts))
  (bind _returnvalue (Utilities|Array|Length _playerstarts))
  (bind _returnvalue_2 (- _returnvalue 1))
  (bind _returnvalue_3 (Math|Random|RandomIntegerinRange 0 _returnvalue_2))
  (bind _output (Utilities|Array|Get(acopy) _playerstarts _returnvalue_3))
  (bind _output_get (LocalVariables|SetPlayerStart _output))
  (while (Variables|/Game/Blueprints/BP_Trolled_PlayerStart.BP_Trolled_PlayerStart_C|GetUsed _output_get)
    (LocalVariables|SetPlayerStart _output))
  (Default|MarkUsed (LocalVariables|GetPlayerStart))
  (return (LocalVariables|GetPlayerStart)))